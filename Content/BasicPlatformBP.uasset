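; BasicPlatformBP is a platform actor that spins around its vertical axis when switched on.
; StartMoving drives a FlipFlop that toggles the spin on and off.
; While on, Tick adds Speed scaled by delta time to CurHeight, which despite its name serves as the relative yaw.
; BeginPlay saves StartPosition, but nothing here reads it, and the overlap event is empty.
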(event Custom|StartMoving
  ;[1 1 1] Spinning platform
  (bind _isa (Utilities|FlowControl|FlipFlop)))

(event EventBeginPlay
  (Variables|Default|SetStartPosition (Transformation|GetActorLocation)))

(event Collision|EventActorBeginOverlap
  (params (OtherActor :type Actor%20Object%20Reference)))

(event EventTick
  (params (DeltaSeconds :type Float%20%28single-precision%29))
  ;[1 1 1] Spinning platform
  (if (stale Custom|StartMoving _isa)
    (bind _output_get (Variables|Default|SetcurHeight (+ (* DeltaSeconds (Variables|Default|GetSpeed)) (Variables|Default|GetcurHeight))))
    (Transformation|SetActorRelativeRotation (Math|Rotator|MakeRotator 0.0 0.0 _output_get))))

(fn ConstructionScript)