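; Physics-driven hover actor that floats its static mesh using downward-tracing thruster components.
; BeginPlay gathers the PhysicsThruster components and applies linear and angular damping to steady the body.
; Each Tick, every thruster traces along the mesh's down axis for twice Height, scaling thrust inversely with hit distance.
; A missed trace leaves that thruster's active state and last strength unchanged.
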(event EventBeginPlay
  (bind _staticmeshcomponent (Variables|Debug|GetStaticMeshComponent))
  (Variables|Default|SetThrusters (Actor|GetComponentsByClass "/Script/Engine.PhysicsThrusterComponent"))
  (Class|PrimitiveComponent|SetLinearDamping _staticmeshcomponent 5.0)
  (Class|PrimitiveComponent|SetAngularDamping _staticmeshcomponent 2e+01))

(event Collision|EventActorBeginOverlap
  (params (OtherActor :type Actor%20Object%20Reference)))

(event EventTick
  (params (DeltaSeconds :type Float%20%28single-precision%29))
  (for _array_element (Variables|Default|GetThrusters)
    (bind (_outhit _returnvalue) (Collision|LineTraceForObjects (Transformation|GetWorldLocation _array_element) (+ (Transformation|GetWorldLocation _array_element) (Math|Vector|NegateVector (* (Math|Vector|GetUpVector (Variables|Debug|GetStaticMeshComponent)) (* (Variables|Default|GetHeight) 2.0)))) (Variables|Default|GetObjects) false 0 "ForOneFrame"))
    (if _returnvalue
      (Components|Activation|SetActive _array_element _returnvalue false)
      (Variables|/Script/Engine.PhysicsThrusterComponent|SetThrustStrength _array_element (* (Variables|Default|GetMaxPower) (/ (Variables|Default|GetHeight) (Math|Float|Max(Float) (.Distance (Collision|BreakHitResult _outhit)) 0.05)))))))

(fn ConstructionScript)