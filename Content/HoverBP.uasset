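; HoverBP is a component that makes its owner hover over surfaces using physics forces.
; Each tick it traces along the owner's downward axis for twice the hover height.
; On a hit, it pushes the static mesh along the surface normal, scaled by mass, gravity and power, growing stronger as distance shrinks.
; Damping rises near ground and drops otherwise; the trace and force are shown for debugging.
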(event EventBeginPlay)

(event EventTick
  (params (DeltaSeconds :type Float%20%28single-precision%29))
  (bind _returnvalue (Components|GetOwner))
  (bind _returnvalue_2 (Components|GetOwner))
  (bind _returnvalue_3 (Actor|GetComponentbyClass _returnvalue_2 "/Script/Engine.StaticMeshComponent"))
  (bind _returnvalue_4 (Transformation|GetActorLocation _returnvalue))
  (bind (_outhit _returnvalue_5) (Collision|LineTraceForObjects _returnvalue_4 (+ _returnvalue_4 (* (Math|Vector|NegateVector (Transformation|GetActorUpVector _returnvalue)) (* (Variables|Default|GetHeight) 2.0))) (Variables|Default|GetObjects) false 0 "ForOneFrame"))
  (if _returnvalue_5
    (Class|PrimitiveComponent|SetLinearDamping _returnvalue_3 5.0)
    (Class|PrimitiveComponent|SetAngularDamping _returnvalue_3 5.0)
    (Physics|AddForce _returnvalue_3 (* (.Normal (Collision|BreakHitResult _outhit)) (* (* (Variables|Default|GetGravity) (Variables|Default|GetPower) (Physics|GetMass _returnvalue_3)) (/ (Variables|Default|GetHeight) (Math|Float|Max(Float) (.Distance (Collision|BreakHitResult _outhit)) 1e+01)))) "None" false)
    (Development|PrintString (Utilities|String|ToString(Text) (Utilities|Text|FormatText "{Force}" (* (* (Variables|Default|GetGravity) (Variables|Default|GetPower) (Physics|GetMass _returnvalue_3)) (/ (Variables|Default|GetHeight) (Math|Float|Max(Float) (.Distance (Collision|BreakHitResult _outhit)) 1e+01))))))
    (else
      (Class|PrimitiveComponent|SetLinearDamping _returnvalue_3 1.0)
      (Class|PrimitiveComponent|SetAngularDamping _returnvalue_3 1.0))))